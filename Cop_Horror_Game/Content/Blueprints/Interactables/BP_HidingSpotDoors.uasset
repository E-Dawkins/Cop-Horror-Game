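; BP_HidingSpotDoors is an interactable double-door hiding spot that the player can open and close.
; A box overlap shows the "to hide" prompt and enables the Interact input for the player character.
; Interacting toggles IsOpen, fires the Interact event with it, and plays both door animations forward or in reverse based on playback position.
; Input locks during the swing until Tick detects the left door at either endpoint.
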(event `self.ReceiveBeginPlay`
  (bind _returnvalue (`|CreateWidget` "/Game/Blueprints/UI/WBP_Interactable.WBP_Interactable_C" (`GameplayStatics.GetPlayerController` 0)))
  (bind _output_get (set `self.InteractUI` _returnvalue))
  (`/Game/Blueprints/UI/WBP_Interactable.Set Hint Text` _output_get "to hide"))

(event `self.Box.OnComponentBeginOverlap`
  (params (OverlappedComponent :type "PrimitiveComponent Object Reference") (OtherActor :type "Actor Object Reference") (OtherComp :type "PrimitiveComponent Object Reference") (OtherBodyIndex :type Integer) (bFromSweep :type Boolean) (SweepResult :type "HitResult Structure (by ref)"))
  (cast `/Game/Blueprints/BP_PlayerCharacter` OtherActor)
  (`UserWidget.AddToViewport` (`self.InteractUI`) 0)
  (set `self.CanInteract` true))

(event `self.Box.OnComponentEndOverlap`
  (params (OverlappedComponent :type "PrimitiveComponent Object Reference") (OtherActor :type "Actor Object Reference") (OtherComp :type "PrimitiveComponent Object Reference") (OtherBodyIndex :type Integer))
  (cast `/Game/Blueprints/BP_PlayerCharacter` OtherActor)
  (`Widget.RemoveFromParent` (`self.InteractUI`))
  (set `self.CanInteract` false))

(event `EnhancedInput|/Game/Input/IA_Interact`
  (params (ActionValue :type Boolean) (ElapsedSeconds :type "Float (double-precision)") (TriggeredSeconds :type "Float (double-precision)") (InputAction :type "InputAction Object Reference" :default "/Game/Input/IA_Interact.IA_Interact"))
  (bind _doorl (`self.DoorL`))
  (bind _doorr (`self.DoorR`))
  (bind _doorl_2 (`self.DoorL`))
  (bind _doorr_2 (`self.DoorR`))
  (:`Triggered`
    (if (`self.CanInteract`)
      (set `self.CanInteract` false)
      (bind _output_get (set `self.IsOpen` (not (`self.IsOpen`))))
      (`self.InteractEvent` _output_get)
      (if (== 0.0 (`SkeletalMeshComponent.GetPosition` (`self.DoorL`)))
        (`SkeletalMeshComponent.SetPlayRate` _doorl_2 1.0)
        (`SkeletalMeshComponent.Play` _doorl_2 false)
        (`SkeletalMeshComponent.SetPlayRate` _doorr_2 1.0)
        (`SkeletalMeshComponent.Play` _doorr_2 false)
        (else
          (`SkeletalMeshComponent.SetPlayRate` _doorl -1.0)
          (`SkeletalMeshComponent.Play` _doorl false)
          (`SkeletalMeshComponent.SetPlayRate` _doorr -1.0)
          (`SkeletalMeshComponent.Play` _doorr false))))))

(event `self.ReceiveTick`
  (params (DeltaSeconds :type "Float (single-precision)"))
  (bind _doorl (`self.DoorL`))
  (bind _doorl_2 (`self.DoorL`))
  ; Check if we can re-interact with the hiding spot
  (if (or (and (`SkeletalMeshComponent.IsPlaying` _doorl_2) (== 0.0 (`SkeletalMeshComponent.GetPosition` _doorl_2))) (and (`SkeletalMeshComponent.IsPlaying` _doorl) (== 1.0 (`SkeletalMeshComponent.GetPosition` _doorl))))
    (set `self.CanInteract` true)))

(fn `UserConstructionScript`
  (`parent.UserConstructionScript`))