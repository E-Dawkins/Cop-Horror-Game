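; Interactable hinged door that toggles open and closed when interacted with.
; A FlipFlop plays or reverses the DoorOpen timeline, driving the door's yaw up to 90 degrees and switching the hint text.
; Opening direction comes from the dot product of door and player forward vectors, so it depends on the player's facing; closing keeps the current yaw sign.
; Interaction is disabled until the timeline finishes.
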(event `self.OnInteract`
  (if (`self.Get Can Interact`)
    (`self.Set Can Interact` false)
    (bind _isa (`/Engine/EditorBlueprintResources/StandardMacros.FlipFlop`)
      (:`A`
        (bind (_direction _doortimer) (`Timeline|DoorOpen` :!label _label)
          (:`Update`
            (`self.Set Interaction Text` _isa)
            (bind _returnvalue (`self.Get Door Angle Sign` _isa))
            (`SceneComponent.K2_SetRelativeRotation` (`self.Door`) (`KismetMathLibrary.MakeRotator` 0.0 0.0 (* _returnvalue 90.0 _doortimer)) false false))
          (:`Finished`
            (`self.Set Can Interact` true))))
      (:`B`
        (goto _label :!via `Reverse`)))))

(fn `Get Door Angle Sign`
  (params (bIsOpen :type Boolean))
  (returns (ReturnValue :type "Float (double-precision)"))
  (bind (_relativerotation_roll _relativerotation_pitch _relativerotation_yaw) (`KismetMathLibrary.BreakRotator` (`SceneComponent.RelativeRotation` (`self.Door`))))
  (if bIsOpen
    (return (`KismetMathLibrary.SignOfFloat` (`KismetMathLibrary.Dot_VectorVector` (`KismetMathLibrary.Conv_RotatorToVector` (`self.K2_GetActorRotation`)) (`KismetMathLibrary.Conv_RotatorToVector` (`self.K2_GetActorRotation` (`GameplayStatics.GetPlayerCharacter` 0))))))
    (else
      (return (`KismetMathLibrary.SignOfFloat` _relativerotation_yaw)))))

(fn `Set Interaction Text`
  (params (bIsOpen :type Boolean))
  (if bIsOpen
    (set `self.HintText` "to close")
    (else
      (set `self.HintText` "to open"))))

(fn `UserConstructionScript`
  (`parent.UserConstructionScript`))