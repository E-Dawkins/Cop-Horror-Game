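; BP_HidingSpot is an interactable that moves the player character into and out of a hiding place.
; It listens to the interact event of its child door actor, then plays or reverses a timeline that lerps the player between their starting transform and the camera-offset Enter point.
; Entering swaps input mapping contexts and disables movement and controller-driven rotation; these are restored once the reverse movement finishes.
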(event `self.ReceiveBeginPlay`
  (bind _asbp_hiding_spot_doors (cast `/Game/Blueprints/Interactables/BP_HidingSpotDoors` (`ChildActorComponent.ChildActor` (`self.BP_HidingSpotDoors`))))
  (add `/Game/Blueprints/Interactables/BP_HidingSpotDoors.InteractEvent` _asbp_hiding_spot_doors (delegate `OnInteract`)))

(event `OnInteract`
  (params (IsOpen :type Boolean))
  (if IsOpen
    (bind (_direction _percent) (`Timeline|Timeline` :!via `ReverseFromEnd` :!label _label)
      (:`Update`
        (bind (_returnvalue_location _returnvalue_rotation) (`KismetMathLibrary.BreakTransform` (`KismetMathLibrary.TLerp` (`self.InitialTransform`) (`self.TargetTransform`) _percent)))
        (`self.K2_SetActorLocationAndRotation` (`GameplayStatics.GetPlayerCharacter` 0) _returnvalue_location _returnvalue_rotation false false))
      (:`Finished`
        (switch `ETimelineDirection` _direction
          (:`Backward`
            (`self.OnExitHide`)))))
    (else
      (`self.OnEnterHide`)
      (goto _label :!via `PlayFromStart`))))

(fn `OnEnterHide`
  (locals (BP_PlayerCharacter :type "/Game/Blueprints/BP_PlayerCharacter Object Reference"))
  (bind _bp_playercharacter (`local.BP_PlayerCharacter`))
  (bind (_returnvalue_location _returnvalue_rotation) (`KismetMathLibrary.BreakTransform` (`self.GetTransform` (`local.BP_PlayerCharacter`))))
  (bind (_returnvalue_location_2 _returnvalue_rotation_2) (`KismetMathLibrary.BreakTransform` (`SceneComponent.K2_GetComponentToWorld` (`self.Enter`))))
  (bind _returnvalue (pcsubsystem `EnhancedInputLocalPlayerSubsystem` (`GameplayStatics.GetPlayerController` 0)))
  ; Store BP_PlayerCharacter
  (bind _asbp_player_character (cast `/Game/Blueprints/BP_PlayerCharacter` (`GameplayStatics.GetPlayerCharacter` 0)))
  (set `local.BP_PlayerCharacter` _asbp_player_character)
  ; Store the initial and target transforms
  (set `self.InitialTransform` (`KismetMathLibrary.MakeTransform` _returnvalue_location _returnvalue_rotation))
  (set `self.TargetTransform` (`KismetMathLibrary.MakeTransform` (- _returnvalue_location_2 (`SceneComponent.RelativeLocation` (`/Game/Blueprints/BP_PlayerCharacter.Camera` (`local.BP_PlayerCharacter`)))) _returnvalue_rotation_2))
  ; Swap input mappings
  (`EnhancedInputSubsystemInterface.RemoveMappingContext` _returnvalue "/Game/Input/IMC_PlayerCharacter.IMC_PlayerCharacter" (struct))
  (`EnhancedInputSubsystemInterface.AddMappingContext` _returnvalue "/Game/Input/IMC_HidingSpot.IMC_HidingSpot" 0 (struct))
  ; Disable movement & bUsePawnControlRotation
  (`CharacterMovementComponent.DisableMovement` (`Character.CharacterMovement` _bp_playercharacter))
  (set `Pawn.bUseControllerRotationYaw` false _bp_playercharacter)
  (set `CameraComponent.bUsePawnControlRotation` false (`/Game/Blueprints/BP_PlayerCharacter.Camera` _bp_playercharacter)))

(fn `OnExitHide`
  (locals (BP_PlayerCharacter :type "/Game/Blueprints/BP_PlayerCharacter Object Reference"))
  (bind _bp_playercharacter (`local.BP_PlayerCharacter`))
  (bind _returnvalue (pcsubsystem `EnhancedInputLocalPlayerSubsystem` (`GameplayStatics.GetPlayerController` 0)))
  ; Store BP_PlayerCharacter
  (bind _asbp_player_character (cast `/Game/Blueprints/BP_PlayerCharacter` (`GameplayStatics.GetPlayerCharacter` 0)))
  (set `local.BP_PlayerCharacter` _asbp_player_character)
  ; Swap input mappings
  (`EnhancedInputSubsystemInterface.RemoveMappingContext` _returnvalue "/Game/Input/IMC_HidingSpot.IMC_HidingSpot" (struct))
  (`EnhancedInputSubsystemInterface.AddMappingContext` _returnvalue "/Game/Input/IMC_PlayerCharacter.IMC_PlayerCharacter" 0 (struct))
  ; Disable movement & bUsePawnControlRotation
  (`CharacterMovementComponent.SetMovementMode` (`Character.CharacterMovement` _bp_playercharacter) "MOVE_Walking" 0)
  (set `Pawn.bUseControllerRotationYaw` true _bp_playercharacter)
  (set `CameraComponent.bUsePawnControlRotation` true (`/Game/Blueprints/BP_PlayerCharacter.Camera` _bp_playercharacter)))

(fn `UserConstructionScript`
  (`parent.UserConstructionScript`))